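; Player pawn that launches a ball from a mouse drag.
; On BeginPlay it sets the view to the first BP_Stage, shows the cursor and stores the first BP_Ball as CurrentBall.
; While CanFire is true, left press records the cursor position, and release passes the normalized drag direction, with X negated, to the ball's Fire.
; Firing clears CanFire, and nothing here resets it.
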(event `self.ReceiveBeginPlay`
  (bind _returnvalue (`GameplayStatics.GetPlayerController` 0))
  (`|ExecutionSequence`
    (:`then_0`
      (bind _outactors (`GameplayStatics.GetAllActorsOfClass` "/Game/BP_Stage.BP_Stage_C"))
      (`PlayerController.SetViewTargetWithBlend` _returnvalue (`|GetArrayItem` _outactors) 0.0 "VTBlend_Linear" 0.0 false)
      (set `PlayerController.bShowMouseCursor` true _returnvalue))
    (:`then_1`
      (bind _outactors_2 (`GameplayStatics.GetAllActorsOfClass` "/Game/BP_Ball.BP_Ball_C"))
      (set `self.currentBall` (`|GetArrayItem` _outactors_2)))))

(event `Key|LeftMouseButton`
  (params (Key :type "Key Structure"))
  (bind (_locationx _locationy) (`PlayerController.GetMousePosition` (`GameplayStatics.GetPlayerController` 0)))
  (bind (_locationx_2 _locationy_2) (`PlayerController.GetMousePosition` (`GameplayStatics.GetPlayerController` 0)))
  (bind (_x _y) (`KismetMathLibrary.BreakVector2D` (`KismetMathLibrary.Normal2D` (- (`KismetMathLibrary.MakeVector2D` _locationx _locationy) (`self.pressPosition`)))))
  (:`Pressed`
    (if (`self.canFire`)
      (set `self.pressPosition` (`KismetMathLibrary.MakeVector2D` _locationx_2 _locationy_2))))
  (:`Released`
    (if (`self.canFire`)
      (bind _currentball (`self.currentBall`)
        (:`then`
          (set `self.canFire` false)
          (`/Game/BP_Ball.Fire` _currentball (* _x -1.0) _y))
        (:`else`)))))

(fn `UserConstructionScript`)