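; BP_Enemy is an enemy Blueprint that shows its health through a UI_HP widget.
; On BeginPlay it caches the widget from its WidgetHP component, stores the starting Hp as InitialHP and calls UpdateHP.
; UpdateHP checks that the widget is valid, then sets its percent to current Hp divided by InitialHP.
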(event `self.ReceiveBeginPlay`
  (`|ExecutionSequence`
    (:`then_0`
      (`|ExecutionSequence`
        (:`then_0`
          (bind _asui_hp (cast `/Game/UI_HP` (`WidgetComponent.GetUserWidgetObject` (`self.Widget_HP`))))
          (set `self.UI_HP` _asui_hp))
        (:`then_1`
          (set `self.initialHP` (`self.hp`)))))
    (:`then_1`
      (`self.UpdateHP`))))

(fn `UpdateHP`
  (bind _ui_hp (`self.UI_HP`)
    (:`then`
      (`/Game/UI_HP.SetPercent` _ui_hp (/ (`self.hp`) (`self.initialHP`))))
    (:`else`)))

(fn `UserConstructionScript`)